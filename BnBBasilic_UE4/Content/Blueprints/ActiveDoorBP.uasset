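; ActiveDoorBP is an automatic door that swings when a WalkingCharacter or FlyingCharacter enters its Box trigger and swings back when one leaves.
; Overlap events play or reverse a timeline that yaws the Arrow component up to 90 degrees, with the direction set by the Opening flag at BeginPlay.
; If a head-mounted display is connected, BeginPlay also plays the timeline immediately.
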(event OnComponentBeginOverlap(Box)
  (params (OverlappedComponent :type Primitive%20Component%20Object%20Reference) (OtherActor :type Actor%20Object%20Reference) (OtherComp :type Primitive%20Component%20Object%20Reference) (OtherBodyIndex :type Integer) (bFromSweep :type Boolean) (SweepResult :type Hit%20Result%20Structure%20%28by%20ref%29))
  ;[1 1 1] Something hit the door...
  (Utilities|Casting|CastToWalkingCharacter OtherActor
    (:then
      ;[1 1 1] It was charecter - start to animate
      (bind _newtrack_4 (Timeline|Timeline_Rotate Play)
        (:Update
          (Transformation|SetRelativeRotation (Variables|Default|GetArrow) (Math|Rotator|MakeRotator 0.0 0.0 (* _newtrack_4 (Variables|Default|GetLimmit))) false false))))
    (:CastFailed
      (Utilities|Casting|CastToFlyingCharacter OtherActor)
      (Timeline|Timeline_Rotate Play))))

(event OnComponentEndOverlap(Box)
  (params (OverlappedComponent :type Primitive%20Component%20Object%20Reference) (OtherActor :type Actor%20Object%20Reference) (OtherComp :type Primitive%20Component%20Object%20Reference) (OtherBodyIndex :type Integer))
  ;[1 1 1] Something hit the door...
  (Utilities|Casting|CastToWalkingCharacter OtherActor
    (:then
      ;[1 1 1] It was charecter - start to animate
      (bind _newtrack_4 (Timeline|Timeline_Rotate Reverse)
        (:Update
          (Transformation|SetRelativeRotation (Variables|Default|GetArrow) (Math|Rotator|MakeRotator 0.0 0.0 (* _newtrack_4 (Variables|Default|GetLimmit))) false false))))
    (:CastFailed
      (Utilities|Casting|CastToFlyingCharacter OtherActor)
      (Timeline|Timeline_Rotate Reverse))))

(event EventBeginPlay
  ;[1 1 1] Is this door openeabele or closable
  (Utilities|FlowControl|Sequence
    (:then_0
      (if (Class|HeadMountedDisplayFunctionLibrary|IsHeadMountedDisplayConnected)
        ;[1 1 1] It was charecter - start to animate
        (bind _newtrack_4 (Timeline|Timeline_Rotate Play)
          (:Update
            (Transformation|SetRelativeRotation (Variables|Default|GetArrow) (Math|Rotator|MakeRotator 0.0 0.0 (* _newtrack_4 (Variables|Default|GetLimmit))) false false)))))
    (:then_1
      (if (Variables|Default|GetOpening)
        (Variables|Default|SetLimmit 9e+01)
        (else
          (Variables|Default|SetLimmit -9e+01))))))

(fn ConstructionScript)